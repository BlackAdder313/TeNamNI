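; GameConstants is a central Blueprint of getters for tuning values: oxygen, flashlight battery, player walk and sprint speeds, and enemy AI roaming, sight and movement.
; Most getters return their stored variable directly.
; Enemy sight radius, vision angle, and chase and roam speeds grow 5% per victory, using the Win count from LastSong_GameInstance capped at MaxVictories.
; Roam wait time and random location radius stay unscaled.
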(fn GetMaxOxygen
  (return (LocalVariables|GetMaxO2)))

(fn GetOxygenDepletionIntervalinSeconds
  (return (LocalVariables|GetIntervalInseconds)))

(fn GetOxygenDepletionAmount
  (return (LocalVariables|GetOxygenDepletionAmount)))

(fn GetWaitTimeonRoam
  (return (LocalVariables|GetWaitTimeInSeconds)))

(fn GetRandomLocationRadius
  (return (LocalVariables|GetRandomLocationRadius)))

(fn GetEnemySightRadius
  (return (|(value*(1.000000+(factor*0.050000))) (LocalVariables|GetEnemySightRadius) (Math|Conversions|ToFloat(Integer) (AI|GetAIFactoronVictories)))))

(fn GetEnemyPeripheralVisionAngle
  (return (|(value*(1.000000+(factor*0.050000))) (LocalVariables|GetEnemyVisionAngle) (Math|Conversions|ToFloat(Integer) (AI|GetAIFactoronVictories)))))

(fn GetMaxBattery
  (return (LocalVariables|GetMaxBatteryCharge)))

(fn GetBatteryDepletionIntervalinSeconds
  (return (LocalVariables|GetIntervalInseconds)))

(fn GetBatteryDepletionAmount
  (return (LocalVariables|GetBatteryDepletionAmount)))

(fn GetFlashlightMaxIntensity
  (return (LocalVariables|GetMaxIntensity)))

(fn GetSprintOxygenDepletionIntervalinSeconds
  (return (LocalVariables|GetIntervalInseconds)))

(fn GetSprintSpeed
  (return (LocalVariables|GetSprintSpeed)))

(fn GetWalkingSpeed
  (return (LocalVariables|GetWalkingSpeed)))

(fn GetAIFactoronVictories
  (bind _aslast_song_game_instance (Utilities|Casting|CastToLastSong_GameInstance (Game|GetGameInstance)))
  (return (|(min(value,limit)) (Variables|/Game/Blueprints/Gamemode/LastSong_GameInstance.LastSong_GameInstance_C|GetWin _aslast_song_game_instance) (LocalVariables|GetMax%20Victories))))

(fn GetMonsterChaseMovementSpeed
  (return (|(value*(1.000000+(factor*0.050000))) (LocalVariables|GetChaseSpeed) (Math|Conversions|ToFloat(Integer) (AI|GetAIFactoronVictories)))))

(fn GetMonsterRoamMovementSpeed
  (return (|(value*(1.000000+(factor*0.050000))) (LocalVariables|GetRoamSpeed) (Math|Conversions|ToFloat(Integer) (AI|GetAIFactoronVictories)))))