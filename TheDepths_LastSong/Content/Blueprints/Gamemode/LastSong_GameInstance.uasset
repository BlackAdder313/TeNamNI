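; LastSong game instance that keeps running tallies of player deaths and wins.
; OnDeath and OnWin each update their counter, Deaths or Win, through a math expression node that appears to add one.
; The file shows no saving, reading or resetting of these counters.
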(fn OnDeath
  (Variables|Default|SetDeaths (|(x+1) (Variables|Default|GetDeaths))))

(fn OnWin
  (Variables|Default|SetWin (|(x+1) (Variables|Default|GetWin))))