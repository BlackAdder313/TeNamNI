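; BP_Enemy is an AI-controlled enemy character that hunts and kills the player diver.
; Entering its AttackRange triggers, once, the looping attack animation, the "Caught" music parameter and player dialogue.
; Entering EatingRange unpossesses the enemy, disables player input and triggers player death after a delay.
; Helper functions expose the patrol route, read and write the Blackboard alert state, and set walk speed per movement mode.
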(event OnComponentBeginOverlap(EatingRange)
  (params (OverlappedComponent :type Primitive%20Component%20Object%20Reference) (OtherActor :type Actor%20Object%20Reference) (OtherComp :type Primitive%20Component%20Object%20Reference) (OtherBodyIndex :type Integer) (bFromSweep :type Boolean) (SweepResult :type Hit%20Result%20Structure%20%28by%20ref%29))
  (bind (_asbp_player_diver _bsuccess) (Utilities|Casting|CastToBP_PlayerDiver OtherActor))
  ;[1 1 1] Kills Player (Basic)
  (if _bsuccess
    (Utilities|FlowControl|DoOnce false
      (:Completed
        (CallFunction|OnGameEnd)
        (Input|DisableInput _asbp_player_diver 0)
        (Utilities|FlowControl|Delay 5.0)
        (Default|OnPlayerDeath _asbp_player_diver "NewEnumerator0")))))

(event OnComponentBeginOverlap(AttackRange)
  (params (OverlappedComponent :type Primitive%20Component%20Object%20Reference) (OtherActor :type Actor%20Object%20Reference) (OtherComp :type Primitive%20Component%20Object%20Reference) (OtherBodyIndex :type Integer) (bFromSweep :type Boolean) (SweepResult :type Hit%20Result%20Structure%20%28by%20ref%29))
  (bind (_asbp_player_diver _bsuccess) (Utilities|Casting|CastToBP_PlayerDiver OtherActor))
  ;[1 1 1] Attack Anim Plays when Player in range of Attack Range collision
  (if _bsuccess
    (Utilities|FlowControl|DoOnce false
      (:Completed
        (CallFunction|OnPlayerAttack)
        (Default|OnDialogueTrigger _asbp_player_diver "NewEnumerator1")))))

(event EventBeginPlay
  ;[1 1 1] Simple Anim solution
)

(event Collision|EventActorBeginOverlap
  (params (OtherActor :type Actor%20Object%20Reference)))

(fn ConstructionScript)

(fn OnPlayerAttack
  (Components|Animation|PlayAnimation (Variables|Default|GetSkeletalMesh) "/Game/Blueprints/Enemy/Animation/Attack_Anim_1.Attack_Anim_1" true)
  (Class|FMODAudioComponent|SetParameter (Variables|Default|GetSong%20Music) "Caught" 1.0))

(fn OnGameEnd
  (Pawn|UnPossess (AI|GetAIController self)))

(fn GetEnemyAlertState
  (return (Utilities|Enum|ByteToEnumE_EnemyAlertState (Class|BlackboardComponent|GetValueasEnum (AI|GetBlackboard (AI|GetAIController self)) (Variables|AI|BlackBoardKeys|GetEnemyAlertStateKey)))))

(fn GetPatrolRoute
  (return (Variables|AI|GetPatrolRoute)))

(fn SetEnemyAlertState
  (params (Enemy%20Alert%20State :type E_EnemyAlertState%20Enum :default "NewEnumerator0"))
  (Utilities|IsValid (Variables|AI|GetBlackboard)
    (:Is%20Valid
      _)
    (:Is%20Not%20Valid
      (Variables|AI|SetBlackboard (AI|GetBlackboard (AI|GetAIController self)))))
  (AI|Components|Blackboard|SetValueasEnum (Variables|AI|GetBlackboard) (Variables|AI|BlackBoardKeys|GetEnemyAlertStateKey) Enemy%20Alert%20State)
  (switch Utilities|FlowControl|Switch|SwitchonE_EnemyAlertState Enemy%20Alert%20State))

(fn SetMovementSpeed
  (params (SpeedMode :type E_MovementSpeed%20Enum :default "NewEnumerator0"))
  (bind _output_get (Variables|/Script/Engine.CharacterMovementComponent|SetMaxWalkSpeed (Variables|Character|GetCharacterMovement) (Utilities|Select :Index SpeedMode :NewEnumerator0 2.5e+02 :NewEnumerator1 3.5e+02 :NewEnumerator2 4.5e+02 :NewEnumerator3 5e+01)))
  (return _output_get))