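; BP_PatrolRoute is an enemy AI patrol path that exposes the points of a spline as waypoints.
; GetSplinePointAsWorldPosition returns the world location of the spline point at the current PatrolIndex.
; IncrementPatrolRoute advances that index through a math expression that wraps by the point count, so the route loops.
; The route holds the index itself and has no active event logic, leaving movement to whatever calls these functions.
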(event EventBeginPlay)

(event Collision|EventActorBeginOverlap
  (params (OtherActor :type Actor%20Object%20Reference)))

(event EventTick
  (params (DeltaSeconds :type Float%20%28single-precision%29)))

(fn ConstructionScript)

(fn IncrementPatrolRoute
  (Variables|Default|SetPatrolIndex (|((index+1)%spline_points_num) (Variables|Default|GetPatrolIndex) (Spline|GetNumberOfSplinePoints (Variables|Default|GetPatrolRoute)))))

(fn GetSplinePointasWorldPosition
  (return (Spline|GetLocationatSplinePoint (Variables|Default|GetPatrolRoute) (Variables|Default|GetPatrolIndex) "World")))