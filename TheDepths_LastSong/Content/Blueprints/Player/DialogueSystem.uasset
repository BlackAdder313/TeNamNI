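; DialogueSystem supplies dialogue for introductions, attacks and wins.
; The introduction reads the win count from LastSong_GameInstance, returning the initial dialogue at zero or a dedicated one for each of the first four wins.
; Any other count makes the selector call itself with a random win number, reusing one of those four.
; Attack dialogue is picked randomly from three options, while win dialogue is fixed.
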(fn GetIntroductionDialogue
  (bind _returnvalue (Game|GetGameInstance))
  (bind (_aslast_song_game_instance _bsuccess) (Utilities|Casting|CastToLastSong_GameInstance _returnvalue))
  (bind _win (Variables|/Game/Blueprints/Gamemode/LastSong_GameInstance.LastSong_GameInstance_C|GetWin _aslast_song_game_instance))
  (if _bsuccess
    (if (|(win==0) _win)
      (return (LocalVariables|GetInitialDialogue))
      (else
        (return (Private|GetIntroductionDiologueAfterWin _win))))))

(fn GetIntroductionDiologueAfterWin
  (params (Wins :type Integer))
  (switch int Wins
    (:Default
      (return (Private|GetIntroductionDiologueAfterWin (Math|Random|RandomIntegerinRange 1 4))))
    (:1
      (return (LocalVariables|GetFirstWin)))
    (:2
      (return (LocalVariables|GetSecondWin)))
    (:3
      (return (LocalVariables|GetThirdWin)))
    (:4
      (return (LocalVariables|GetFourthWin)))))

(fn GetAttackDialogue
  (switch int (Math|Random|RandomIntegerinRange 0 2)
    (:Default
      (return (LocalVariables|GetThirdCase)))
    (:0
      (return (LocalVariables|GetFirstCase)))
    (:1
      (return (LocalVariables|GetSecondCase)))))

(fn GetWinDialogue
  (return (LocalVariables|GetWinDialogue)))